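; Interactable security camera console that lets the player view the level's BP_SecurityCamera actors.
; It gathers all cameras at BeginPlay, and Interact toggles viewing by switching input from the character to itself, hiding the main HUD and blocking look input and pausing.
; Space Bar cycles the view target through the cameras with wraparound.
; Return or Action exits, restoring player control, HUD and view and resetting to the first camera.
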(event Custom|LeaveCameraController
  (bind _returnvalue (Game|GetPlayerController 0))
  (Variables|Default|SetisViewingCameras false)
  (Input|DisableInput _returnvalue)
  (Input|ResetIgnoreLookInput _returnvalue)
  (Widget|SetVisibility (Variables|/Game/GameBG/Level1/L1_Character.L1_Character_C|GetMainHudRef (.AsL1%20Character (Utilities|Casting|CastToL1_Character (Game|GetPlayerCharacter 0)))) "SelfHitTestInvisible")
  (Variables|/Game/GameBG/HG_PlayerController.HG_PlayerController_C|SetCanPause (.AsHG%20Player%20Controller (Utilities|Casting|CastToHG_PlayerController (Game|GetPlayerController 0))) true)
  (Input|EnableInput (Game|GetPlayerCharacter 0) (Game|GetPlayerController 0))
  (Variables|Default|SetCarrentCameraIndex 0)
  (Game|Player|SetViewTargetwithBlend (Game|GetPlayerController 0) (Game|GetPlayerCharacter 0) 0.0 "VTBlend_Linear" 0.0 false))

(event EventInteract
  (bind _returnvalue (Game|GetPlayerController 0))
  (if (Variables|Default|GetisViewingCameras)
    (CallFunction|LeaveCameraController)
    (else
      (Variables|Default|SetisViewingCameras true)
      (Input|DisableInput (Game|GetPlayerCharacter 0) _returnvalue)
      (Input|SetIgnoreLookInput _returnvalue true)
      (Widget|SetVisibility (Variables|/Game/GameBG/Level1/L1_Character.L1_Character_C|GetMainHudRef (.AsL1%20Character (Utilities|Casting|CastToL1_Character (Game|GetPlayerCharacter 0)))) "Hidden")
      (Variables|/Game/GameBG/HG_PlayerController.HG_PlayerController_C|SetCanPause (.AsHG%20Player%20Controller (Utilities|Casting|CastToHG_PlayerController (Game|GetPlayerController 0))) false)
      (Input|EnableInput (Game|GetPlayerController 0))
      (CallFunction|ViewThroughCamera))))

(event EventBeginPlay
  (bind _outactors (Actor|GetAllActorsOfClass "/Game/Blueprints/Actors/SecurityCameras/BP_SecurityCamera.BP_SecurityCamera_C"))
  (Variables|Default|SetSecurityCameras _outactors))

(event Input|ActionEvents|InputActionReturn
  (params (Key :type Key%20Structure :default "None"))
  (:Pressed
    (CallFunction|LeaveCameraController)))

(event Input|ActionEvents|InputActionAction
  (params (Key :type Key%20Structure :default "None"))
  (:Pressed
    (CallFunction|LeaveCameraController)))

(event Input|KeyboardEvents|SpaceBar
  (params (Key :type Key%20Structure :default "None"))
  (:Pressed
    (Variables|Default|SetCarrentCameraIndex (select (> (+ (Variables|Default|GetCarrentCameraIndex) 1) (- (Utilities|Array|Length (Variables|Default|GetSecurityCameras)) 1)) 0 (+ (Variables|Default|GetCarrentCameraIndex) 1)))
    (CallFunction|ViewThroughCamera)))

(fn ConstructionScript)

(fn ViewThroughCamera
  (Game|Player|SetViewTargetwithBlend (Game|GetPlayerController 0) (Utilities|Array|Get(acopy) (Variables|Default|GetSecurityCameras) (Variables|Default|GetCarrentCameraIndex)) 0.0 "VTBlend_Linear" 0.0 false)
  (return))
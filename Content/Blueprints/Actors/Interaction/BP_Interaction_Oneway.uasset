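; BP_Interaction_Oneway is an interactable locked door that the player opens with a key and that has no logic to close again.
; BeginPlay caches the player character's inventory component, which Interact searches slot by slot for the referenced key item.
; With the key, a timeline slides the door along X and turns off the Box collision; without it, only a locked-gate sound plays.
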(event EventBeginPlay
  (|CallParentFunction)
  (bind _asl1_character (Utilities|Casting|CastToL1_Character (Game|GetPlayerCharacter 0)))
  (Variables|Default|SetBPC%20Inventory (Variables|/Game/GameBG/Level1/L1_Character.L1_Character_C|GetBPC_Inventory _asl1_character)))

(event Collision|EventActorBeginOverlap
  (params (OtherActor :type Actor%20Object%20Reference)))

(event EventInteract
  (if (Variables|Default|GetIsDoorClosed)
    (CallFunction|CheckHasKey)
    (if (Variables|Default|GetHasKey)
      (Variables|Default|SetIsDoorClosed false)
      (Audio|PlaySound2D "/Game/Sounds/Gate_Close01_Cue.Gate_Close01_Cue" 1.0 1.0 0.0 0 0)
      (bind _alpha (Timeline|OpenDoorTL Play)
        (:Update
          (Transformation|SetRelativeLocation (Variables|Default|GetDoor) (Math|Vector|MakeVector (Math|Float|Lerp 0.0 -205.0 _alpha) 0.0 0.0) false false)
          (Collision|SetCollisionEnabled (Variables|Default|GetBox) "NoCollision")))
      (else
        (Audio|PlaySound2D "/Game/Sounds/closed_gates_Cue.closed_gates_Cue" 1.0 1.0 0.0 0 0)))))

(fn ConstructionScript
  (|CallParentFunction))

(fn CheckHasKey
  (bind _array_element (Utilities|Array|ForEachLoopwithBreak (Variables|/Game/Blueprints/BlueprintComponents/BPC_Inventory.BPC_Inventory_C|GetInventorySlots (Variables|Default|GetBPC%20Inventory)) :!label _label)
    (:LoopBody
      (if (== (.Item (Utilities|Struct|BreakS_InventoryItems _array_element)) (Variables|Default|GetBP_DoorKeyRef))
        (Development|PrintString "have key")
        (goto _label Break)
        (else
          (Development|PrintString "do not have key"))))
    (:Completed
      (Variables|Default|SetHasKey (== (.Item (Utilities|Struct|BreakS_InventoryItems _array_element)) (Variables|Default|GetBP_DoorKeyRef))))))
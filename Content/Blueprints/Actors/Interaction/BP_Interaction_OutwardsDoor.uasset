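; BP_Interaction_OutwardsDoor is an interactable swinging door that opens away from whoever opens it, player or AI.
; Interact toggles it on a timeline, using a dot product against the door's forward vector to pick the swing side.
; AI_Classic overlapping the Box opens it on a separate timeline and blocks interaction until it closes again.
; SetHasKey checks the player's inventory for the key, but Interact ignores the result.
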(event OnComponentBeginOverlap(Box)
  (params (OverlappedComponent :type Primitive%20Component%20Object%20Reference) (OtherActor :type Actor%20Object%20Reference) (OtherComp :type Primitive%20Component%20Object%20Reference) (OtherBodyIndex :type Integer) (bFromSweep :type Boolean) (SweepResult :type Hit%20Result%20Structure%20%28by%20ref%29))
  (bind _self self)
  (bind _asai_classic (Utilities|Casting|CastToAI_Classic OtherActor))
  (Variables|Default|SetcanInteract false)
  (if (Variables|Default|GetIsDoorClosed)
    (Variables|Default|SetIsDoorClosed false)
    (Variables|Default|SetDotProduct (Math|Vector|DotProduct (Math|Vector|Normalize (- (Transformation|GetActorLocation _self) (Transformation|GetActorLocation _asai_classic))) (Transformation|GetActorForwardVector _self)))
    (bind (_direction _alpha) (Timeline|OpenDoorAI PlayFromStart)
      (:Update
        (Transformation|SetRelativeRotation (Variables|Default|GetDoor) (Math|Rotator|MakeRotator 0.0 0.0 (Math|Float|Lerp 0.0 (select (>= (Variables|Default|GetDotProduct) 0.0) 9e+01 -9e+01) _alpha)) false false))
      (:Finished
        (switch Utilities|FlowControl|Switch|SwitchonETimelineDirection _direction
          (:Backward
            (Variables|Default|SetcanInteract true)))))))

(event OnComponentEndOverlap(Box)
  (params (OverlappedComponent :type Primitive%20Component%20Object%20Reference) (OtherActor :type Actor%20Object%20Reference) (OtherComp :type Primitive%20Component%20Object%20Reference) (OtherBodyIndex :type Integer))
  (Utilities|Casting|CastToAI_Classic OtherActor)
  (if (not (Variables|Default|GetIsDoorClosed))
    (Variables|Default|SetIsDoorClosed true)
    (bind (_direction _alpha) (Timeline|OpenDoorAI ReverseFromEnd)
      (:Update
        (Transformation|SetRelativeRotation (Variables|Default|GetDoor) (Math|Rotator|MakeRotator 0.0 0.0 (Math|Float|Lerp 0.0 (select (>= (Variables|Default|GetDotProduct) 0.0) 9e+01 -9e+01) _alpha)) false false))
      (:Finished
        (switch Utilities|FlowControl|Switch|SwitchonETimelineDirection _direction
          (:Backward
            (Variables|Default|SetcanInteract true)))))))

(event EventBeginPlay
  (|CallParentFunction) ; This node is disabled and will not be called.\nDrag off pins to build functionality.
)

(event Collision|EventActorBeginOverlap
  (params (OtherActor :type Actor%20Object%20Reference)))

(event EventInteract
  (bind _self self)
  (if (Variables|Default|GetcanInteract)
    (if (Variables|Default|GetIsDoorClosed)
      (Variables|Default|SetIsDoorClosed false)
      (Variables|Default|SetDotProduct (Math|Vector|DotProduct (Math|Vector|Normalize (- (Transformation|GetActorLocation _self) (Transformation|GetActorLocation (Variables|Default|GetPlayerRef)))) (Transformation|GetActorForwardVector _self)))
      (bind _alpha (Timeline|OpenDoorTL PlayFromStart)
        (:Update
          (Transformation|SetRelativeRotation (Variables|Default|GetDoor) (Math|Rotator|MakeRotator 0.0 0.0 (Math|Float|Lerp 0.0 (select (>= (Variables|Default|GetDotProduct) 0.0) 9e+01 -9e+01) _alpha)) false false)))
      (else
        (Variables|Default|SetIsDoorClosed true)
        (Timeline|OpenDoorTL ReverseFromEnd)))))

(fn ConstructionScript
  (|CallParentFunction))

(fn SetHasKey
  (bind _asl1_character (Utilities|Casting|CastToL1_Character (Game|GetPlayerCharacter 0)))
  (bind _array_element (Utilities|Array|ForEachLoopwithBreak (Variables|/Game/Blueprints/BlueprintComponents/BPC_Inventory.BPC_Inventory_C|GetInventorySlots (Variables|/Game/GameBG/Level1/L1_Character.L1_Character_C|GetBPC_Inventory _asl1_character)) :!label _label)
    (:LoopBody
      (if (== (.Item (Utilities|Struct|BreakS_InventoryItems _array_element)) (Variables|Default|GetBP_DoorKeyRef))
        (Development|PrintString "have key")
        (goto _label Break)
        (else
          (Development|PrintString "do not have key"))))
    (:Completed
      (Variables|Default|SetHasKey (== (.Item (Utilities|Struct|BreakS_InventoryItems _array_element)) (Variables|Default|GetBP_DoorKeyRef))))))
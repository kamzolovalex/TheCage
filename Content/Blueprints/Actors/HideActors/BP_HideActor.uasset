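; BP_HideActor is an interactable hiding spot that moves the player in and out of hiding.
; Interact starts a looping timer that slides the player at constant speed to PlayerPosition or ExitPosition, based on IsHiding.
; Entering disables collision, movement and inventory and asks the AIC_Classic enemy controller whether it saw the player.
; On arrival it fires a dispatcher and toggles IsHiding; exiting also restores control and notifies the AI.
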(event Custom|MoveCharacter
  (bind _playerref (Variables|Default|GetPlayerRef))
  (Transformation|SetActorTransform _playerref (Math|Transform|MakeTransform (Math|Interpolation|VInterptoConstant (Transformation|GetActorLocation _playerref) (Transformation|GetWorldLocation (select (Variables|/Game/GameBG/Level1/L1_Character.L1_Character_C|GetisHiding (Variables|Default|GetPlayerRef)) (Variables|Default|GetExitPosition) (Variables|Default|GetPlayerPosition))) (Utilities|Time|GetWorldDeltaSeconds) 1e+03) "0.000000,90.000000,0.000000" "1,1,1"))
  (if (Math|Vector|Equal(Vector) (Transformation|GetActorLocation (Variables|Default|GetPlayerRef)) (Transformation|GetWorldLocation (select (Variables|/Game/GameBG/Level1/L1_Character.L1_Character_C|GetisHiding (Variables|Default|GetPlayerRef)) (Variables|Default|GetExitPosition) (Variables|Default|GetPlayerPosition))) 0.01)
    (Utilities|Time|ClearandInvalidateTimerbyHandle (stale EventInteract _returnvalue_3))
    (Utilities|Time|ClearandInvalidateTimerbyHandle (stale EventInteract _returnvalue))
    (CallFunction|FinishedMoving)))

(event Custom|FinishedMoving
  (bind _playerref (Variables|Default|GetPlayerRef))
  (bind _playerref_2 (Variables|Default|GetPlayerRef))
  (Default|CallFinishedMovingED)
  (if (Variables|/Game/GameBG/Level1/L1_Character.L1_Character_C|GetisHiding (Variables|Default|GetPlayerRef))
    (Variables|/Game/GameBG/Level1/L1_Character.L1_Character_C|SetisHiding _playerref false)
    (bind _asaic_classic (Utilities|Casting|CastToAIC_ClassicClass "/Game/AI/Classic/AIC_Classic.AIC_Classic_C"))
    (bind _returnvalue (Actor|GetActorOfClass _asaic_classic))
    (Class|BPIPlayerHiding|LeftHidingSpot(Message) _returnvalue)
    (Collision|SetActorEnableCollision _playerref_2 true)
    (Pawn|Components|CharacterMovement|SetMovementMode (Variables|/Script/Engine.Character|GetCharacterMovement _playerref_2) "MOVE_Walking" 0)
    (Variables|/Game/GameBG/Level1/L1_PlayerController.L1_PlayerController_C|SetCanOpenInventory (Variables|Default|GetControllerRef) true)
    (else
      (Variables|/Game/GameBG/Level1/L1_Character.L1_Character_C|SetisHiding _playerref true))))

(event Custom|EnemyFound)

(event EventBeginPlay
  (bind _asl1_character (Utilities|Casting|CastToL1_Character (Game|GetPlayerCharacter 0)))
  (Variables|Default|SetPlayerRef _asl1_character)
  (bind _ashg_player_controller (Utilities|Casting|CastToL1_PlayerController (Game|GetPlayerController 0)))
  (Variables|Default|SetControllerRef _ashg_player_controller))

(event EventInteract
  (bind _playerref (Variables|Default|GetPlayerRef))
  (if (Variables|/Game/GameBG/Level1/L1_Character.L1_Character_C|GetisHiding (Variables|Default|GetPlayerRef))
    (bind _returnvalue (Utilities|Time|SetTimerbyEvent (delegate Custom|MoveCharacter) (Utilities|Time|GetWorldDeltaSeconds) true))
    (else
      (bind _asaic_classic (Utilities|Casting|CastToAIC_ClassicClass "/Game/AI/Classic/AIC_Classic.AIC_Classic_C"))
      (bind _returnvalue_2 (Actor|GetActorOfClass _asaic_classic))
      (Class|BPIPlayerHiding|DidEnemySee(Message) _returnvalue_2 self)
      (Collision|SetActorEnableCollision _playerref false)
      (Pawn|Components|CharacterMovement|DisableMovement (Variables|/Script/Engine.Character|GetCharacterMovement _playerref))
      (Variables|/Game/GameBG/Level1/L1_PlayerController.L1_PlayerController_C|SetCanOpenInventory (Variables|Default|GetControllerRef) false)
      (bind _returnvalue_3 (Utilities|Time|SetTimerbyEvent (delegate Custom|MoveCharacter) (Utilities|Time|GetWorldDeltaSeconds) true)))))

(fn ConstructionScript)
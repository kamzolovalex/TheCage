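; BP_PainRoom_Master is a pain-volume actor that deals periodic damage to an L1_Character inside it.
; The construction script sizes the PainCausing box from RoomSize.
; Overlapping the box stores the player and starts a one-second looping timer that removes Damage through the character's BPCHealth component.
; The timer is cleared when health reaches zero or the character leaves the box.
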(event OnComponentBeginOverlap(PainCausing)
  (params (OverlappedComponent :type Primitive%20Component%20Object%20Reference) (OtherActor :type Actor%20Object%20Reference) (OtherComp :type Primitive%20Component%20Object%20Reference) (OtherBodyIndex :type Integer) (bFromSweep :type Boolean) (SweepResult :type Hit%20Result%20Structure%20%28by%20ref%29))
  (bind _asl1_character (Utilities|Casting|CastToL1_Character OtherActor))
  (Variables|Default|SetPlayerRef _asl1_character)
  (Utilities|Time|SetTimerbyFunctionName 0 "CausePain" 1.0 true))

(event OnComponentEndOverlap(PainCausing)
  (params (OverlappedComponent :type Primitive%20Component%20Object%20Reference) (OtherActor :type Actor%20Object%20Reference) (OtherComp :type Primitive%20Component%20Object%20Reference) (OtherBodyIndex :type Integer))
  (Utilities|Casting|CastToL1_Character OtherActor)
  (Utilities|Time|ClearTimerbyFunctionName 0 "CausePain"))

(event Custom|CausePain
  (bind _playerref (Variables|Default|GetPlayerRef))
  (bind _bpc_health (Variables|/Game/GameBG/Level1/L1_Character.L1_Character_C|GetBPC_Health _playerref))
  (Default|RemoveHealth _bpc_health (Variables|Default|GetDamage))
  (if (<= (Variables|/Game/Blueprints/BlueprintComponents/BPC_Health.BPC_Health_C|GetCurrentHealth _bpc_health) 0.0)
    (Utilities|Time|ClearTimerbyFunctionName 0 "CausePain")))

(event EventBeginPlay)

(event Collision|EventActorBeginOverlap
  (params (OtherActor :type Actor%20Object%20Reference)))

(event EventTick
  (params (DeltaSeconds :type Float%20%28single-precision%29)))

(fn ConstructionScript
  (Components|Box|SetBoxExtent (Variables|Default|GetPainCausing) (Variables|Default|GetRoom%20Size) true))
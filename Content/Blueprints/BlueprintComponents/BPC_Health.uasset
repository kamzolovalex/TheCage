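; Health component for the player that tracks clamped health and triggers game over when it reaches zero.
; Each health change maps health into the MPC_BloodScreen parameter collection, so the blood overlay only appears below roughly 70%.
; Death disables L1_Character movement and input, shows the W_GameOver widget with UI-only input, and destroys all AI_Classic actors, repeating that cleanup after a one-second delay.
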(event Custom|PlayerDied
  (CallFunction|PlayerDeath)
  (Utilities|FlowControl|Delay 1.0)
  (bind _outactors (Actor|GetAllActorsOfClass "/Game/AI/Classic/AI_Classic.AI_Classic_C"))
  (for _array_element _outactors
    (Actor|DestroyActor _array_element)))

(event EventBeginPlay
  (CallFunction|UpdateBloodScreen))

(event EventTick
  (params (DeltaSeconds :type Float%20%28single-precision%29)))

(fn RemoveHealth
  (params (Amount :type Float%20%28single-precision%29))
  (Variables|Default|SetCurrentHealth (Math|Float|Clamp(Float) (- (Variables|Default|GetCurrentHealth) Amount) (Variables|Default|GetMinHealth) (Variables|Default|GetMaxHealth)))
  (CallFunction|UpdateBloodScreen)
  (if (<= (Variables|Default|GetCurrentHealth) 0.0)
    (CallFunction|PlayerDied)))

(fn AddHealth
  (params (Amount :type Float%20%28single-precision%29))
  (Variables|Default|SetCurrentHealth (Math|Float|Clamp(Float) (+ Amount (Variables|Default|GetCurrentHealth)) (Variables|Default|GetMinHealth) (Variables|Default|GetMaxHealth)))
  (CallFunction|UpdateBloodScreen))

(fn UpdateBloodScreen
  (Rendering|Material|SetScalarParameterValue "/Game/Materials/MPC_BloodScreen.MPC_BloodScreen" "Amount" (Math|Float|MapRangeClamped (Variables|Default|GetCurrentHealth) (Variables|Default|GetMinHealth) (* (- (Variables|Default|GetMaxHealth) (Variables|Default|GetMinHealth)) 0.7) 0.5 1.0) :!class /Script/Engine.KismetMaterialLibrary))

(fn PlayerDeath
  (bind _returnvalue (Game|GetPlayerController 0))
  (bind _returnvalue_2 (Game|GetPlayerController 0))
  (Variables|Default|SetIsDying true)
  (bind _asl1_character (Utilities|Casting|CastToL1_Character (Game|GetPlayerCharacter 0)))
  (Pawn|Components|CharacterMovement|DisableMovement (Variables|/Script/Engine.Character|GetCharacterMovement _asl1_character))
  (Input|DisableInput _asl1_character _returnvalue_2)
  (Input|SetIgnoreLookInput _returnvalue_2 true)
  (bind _returnvalue_3 (UserInterface|CreateWidget "/Game/UMG/W_GameOver.W_GameOver_C"))
  (UserInterface|Viewport|AddtoViewport _returnvalue_3 0)
  (Variables|/Script/Engine.PlayerController|SetbShowMouseCursor _returnvalue true)
  (Input|SetInputModeUIOnly _returnvalue _returnvalue_3 "DoNotLock")
  (bind _outactors (Actor|GetAllActorsOfClass "/Game/AI/Classic/AI_Classic.AI_Classic_C"))
  (for _array_element _outactors
    (Actor|DestroyActor _array_element)))